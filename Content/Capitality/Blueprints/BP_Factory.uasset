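; BP_Factory is the factory actor that builds a square floor grid and seeds it with starting blocks.
; On BeginPlay it adds child actor components at regular spacing across FloorSize, then spawns Source, FactoryController and Sink blocks at fixed offsets from its location.
; It also tracks the last control panel, closing it when a different one is passed in, and offers a cleanup that destroys and clears its Props.
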(event `self.ReceiveBeginPlay`
  (`self.InitializeFactoryFloor`))

(fn `CleanUp`
  (bind _props (`self.Props`))
  (`self.K2_DestroyActor` _props)
  (`KismetArrayLibrary.Array_Clear` _props))

(fn `CloseLastControlPanel`
  (params (NewControlPanel :type "/Game/Capitality/Blueprints/BP_FactoryTile Object Reference"))
  (bind _lastcontrolpanel (`self.LastControlPanel`))
  (`/Engine/EditorBlueprintResources/StandardMacros.IsValid` _lastcontrolpanel
    (:`Is Valid`
      (if (!= NewControlPanel _lastcontrolpanel)
        (`/Game/Capitality/Blueprints/BP_FactoryTile.Close` _lastcontrolpanel)))
    (:`Is Not Valid`
      _))
  (set `self.LastControlPanel` NewControlPanel))

(fn `InitializeFactoryFloor`
  (bind _returnvalue (- (`self.FloorSize`) 1))
  (for _index (range (+ _returnvalue 1))
    (for _index_2 (range (+ _returnvalue 1))
      (`AddComponent|NODE_AddChildActorComponent-1` :`RelativeTransform` (`KismetMathLibrary.MakeTransform` (`KismetMathLibrary.MakeVector` (* (`KismetMathLibrary.Conv_IntToDouble` _index_2) 100.0) (* (`KismetMathLibrary.Conv_IntToDouble` _index) 100.0))))))
  (`|SpawnActorFromClass` "/Game/Capitality/Blueprints/BP_Block_Source.BP_Block_Source_C" (`KismetMathLibrary.Conv_VectorToTransform` (+ (`self.K2_GetActorLocation`) (100.0 100.0 0.0))) "Undefined" "OverrideRootScale" null "Source" null)
  (`|SpawnActorFromClass` "/Game/Capitality/Blueprints/BP_Block_FactoryController.BP_Block_FactoryController_C" (`KismetMathLibrary.Conv_VectorToTransform` (+ (`self.K2_GetActorLocation`) (100.0 300.0 0.0))) "Undefined" "OverrideRootScale" null "Controller" null)
  (`|SpawnActorFromClass` "/Game/Capitality/Blueprints/BP_Block_Sink.BP_Block_Sink_C" (`KismetMathLibrary.Conv_VectorToTransform` (+ (`self.K2_GetActorLocation`) (100.0 500.0 0.0))) "Undefined" "OverrideRootScale" null "Sink" null))

(fn `UserConstructionScript`)