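; Bumper block that catches BP_Prop actors entering its Portal and bumps them forward and up.
; A short same-actor debounce guards the overlap, then the prop's velocities are zeroed and it is teleported by a fixed offset, with no physics impulse.
; A bump sound, assigned in the construction script, plays before the empty Process hook receives the prop.
; An unconnected impulse-based version remains, noted as too unreliable for play.
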(event `self.Portal.OnComponentBeginOverlap`
  (params (OverlappedComponent :type "PrimitiveComponent Object Reference") (OtherActor :type "Actor Object Reference") (OtherComp :type "PrimitiveComponent Object Reference") (OtherBodyIndex :type Integer) (bFromSweep :type Boolean) (SweepResult :type "HitResult Structure (by ref)"))
  (if (or (!= OtherActor (`self.LastOverlapper`)) (> (- (`self.GetGameTimeSinceCreation`) (`self.LastOverlapTime`)) 0.05))
    (set `self.LastOverlapper` OtherActor)
    (set `self.LastOverlapTime` (`self.GetGameTimeSinceCreation`))
    (bind _asbp_prop (cast `/Game/Capitality/Blueprints/BP_Prop` OtherActor))
    (bind _staticmeshcomponent (`StaticMeshActor.StaticMeshComponent` _asbp_prop))
    (`PrimitiveComponent.SetPhysicsLinearVelocity` _staticmeshcomponent (0.0 0.0 0.0) false "None")
    (`PrimitiveComponent.SetPhysicsAngularVelocityInRadians` _staticmeshcomponent (0.0 0.0 0.0) false "None")
    (`SceneComponent.K2_AddWorldOffset` _staticmeshcomponent (+ (* (`self.GetActorForwardVector`) 105.0) (0.0 0.0 70.0)) false true)
    (`AudioComponent.Play` (`self.BumpSfx`) 0.0)
    (`self.Process` _asbp_prop)))

(event `self.ReceiveBeginPlay`
  (`parent.ReceiveBeginPlay`))

(fn `Process`
  (params (Prop :type "/Game/Capitality/Blueprints/BP_Prop Object Reference")))

(fn `UserConstructionScript`
  (`parent.UserConstructionScript`)
  (`AudioComponent.SetSound` (`self.BumpSfx`) (`self.Sound`)))