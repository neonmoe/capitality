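; BP_Block_FactoryController is a control block for a factory, with Start, Stop and Clean Up buttons and a stats readout.
; The construction script passes its Factory reference to each BP_Button_FactoryControl child actor.
; Every Tick rewrites StatsText from that Factory's points, operators and transport values, polling rather than reacting to events.
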(event `self.ReceiveTick`
  (params (DeltaSeconds :type "Float (single-precision)"))
  (`parent.ReceiveTick` DeltaSeconds)
  (`self.UpdateStats`))

(fn `SetButtonUp`
  (params (Actor :type "ChildActorComponent Object Reference"))
  (bind _asbp_button_factory_control (cast `/Game/Capitality/Blueprints/BP_Button_FactoryControl` (`ChildActorComponent.ChildActor` Actor)))
  (set `/Game/Capitality/Blueprints/BP_Button_FactoryControl.Factory` (`self.Factory`) _asbp_button_factory_control))

(fn `UpdateStats`
  (bind _factory (`self.Factory`))
  (`TextRenderComponent.K2_SetText` (`self.StatsText`) (`|FormatText` "Points: {Points} \nOperators: {Ops} \nTransport: {Transport}m" (`/Game/Capitality/Blueprints/BP_Factory.Points` _factory) (`/Game/Capitality/Blueprints/BP_Factory.Operators` _factory) (`/Game/Capitality/Blueprints/BP_Factory.Transport` _factory))))

(fn `UserConstructionScript`
  (`parent.UserConstructionScript`)
  (`self.SetButtonUp` (`self.ButtonStart`))
  (`self.SetButtonUp` (`self.ButtonStop`))
  (`self.SetButtonUp` (`self.ButtonCleanUp`)))