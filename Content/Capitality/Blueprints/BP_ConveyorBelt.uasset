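; Conveyor belt actor that lines up static mesh segments toward a configurable end point and spins them.
; The construction script adds meshes from SpawnPoint, stepping ConveyorDistance along the EndPoint direction until reaching that distance from the local origin, all facing along a look-at rotation.
; Tick rotates every stored mesh around its local pitch axis at RotationSpeed, scaled by delta time.
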(event `self.ReceiveTick`
  (params (DeltaSeconds :type "Float (single-precision)"))
  (for _array_element (`self.Conveyors`)
    (`SceneComponent.K2_AddLocalRotation` _array_element (`KismetMathLibrary.MakeRotator` 0.0 (* DeltaSeconds (`self.RotationSpeed`))) false false)))

(fn `UserConstructionScript`
  (locals (SpawnPoint :type "Vector Structure"))
  (set `self.SpawnRotation` (`KismetMathLibrary.FindLookAtRotation` (`self.EndPoint`) (`local.SpawnPoint`)))
  (while (> (`KismetMathLibrary.VSize` (`self.EndPoint`)) (`KismetMathLibrary.VSize` (`local.SpawnPoint`)))
    (`|ExecutionSequence`
      (:`then_0`
        (bind _returnvalue (`AddComponent|NODE_AddStaticMeshComponent-0` :`RelativeTransform` (`KismetMathLibrary.MakeTransform` (`local.SpawnPoint`) (`self.SpawnRotation`))))
        (`KismetArrayLibrary.Array_Add` (`self.Conveyors`) _returnvalue))
      (:`then_1`
        (set `local.SpawnPoint` (+ (`local.SpawnPoint`) (* (`KismetMathLibrary.Normal` (`self.EndPoint`)) (`self.ConveyorDistance`))))))))