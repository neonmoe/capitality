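; BP_Block_Colorer is a block Blueprint that gives a processed prop a random color.
; Its Process event sets the BaseColor vector parameter on the prop's dynamic material instance to random RGB values at full alpha.
; BeginPlay and the construction script only call their parent versions, and the overlap and tick events are inactive.
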(event `self.Process`
  (params (Prop :type "/Game/Capitality/Blueprints/BP_Prop Object Reference"))
  (`MaterialInstanceDynamic.SetVectorParameterValue` (`/Game/Capitality/Blueprints/BP_Prop.DMI` Prop) "BaseColor" (make `LinearColor` (`KismetMathLibrary.RandomFloat`) (`KismetMathLibrary.RandomFloat`) (`KismetMathLibrary.RandomFloat`) 1.0)))

(event `self.ReceiveBeginPlay`
  (`parent.ReceiveBeginPlay`))

(fn `UserConstructionScript`
  (`parent.UserConstructionScript`))