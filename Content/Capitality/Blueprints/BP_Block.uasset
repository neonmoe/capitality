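; BP_Block is an interactable, non-grabbable named block that counts as an operator in BP_Factory and has a pop-up control panel to rotate, delete or close it.
; Being looked at orients and opens the panel, which lerps its scale on Tick and auto-closes after a short timeout.
; Construction finds the factory, links the child-actor buttons back to the block and sets its text labels.
; BeginPlay and Delete adjust the factory's operator count.
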(event `/Game/VRUUM/Blueprints/BPI_Interactible.LookedAt`
  (params (Rotation :type "Rotator Structure"))
  (bind _controlpanel (`self.ControlPanel`))
  (set `self.ControlPanelSize` 1.0)
  (`SceneComponent.SetVisibility` _controlpanel true true)
  (`SceneComponent.SetRelativeScale3D` _controlpanel (0.05 0.05 0.05))
  (`SceneComponent.K2_SetWorldRotation` _controlpanel Rotation false true)
  (set `self.AutocloseTime` (`self.GetGameTimeSinceCreation`)))

(event `self.ReceiveTick`
  (params (DeltaSeconds :type "Float (single-precision)"))
  (`self.UpdateScale` DeltaSeconds)
  (`self.UpdateVisibility`)
  (`self.UpdateAutoclose`))

(event `self.ReceiveBeginPlay`
  (`self.AddOperator`))

(fn `AddOperator`
  (`/Engine/EditorBlueprintResources/StandardMacros.IncrementInt` (`/Game/Capitality/Blueprints/BP_Factory.Operators` (`self.Factory`))))

(fn `CanGrab`
  (returns (Grabbability :type Boolean))
  (return false))

(fn `CanInteract`
  (returns (Interactiblity :type Boolean))
  (return true))

(fn `Close`
  (bind _controlpanel (`self.ControlPanel`))
  (set `self.ControlPanelSize` 0.0)
  (`SceneComponent.SetRelativeScale3D` _controlpanel (0.0 0.0 0.0))
  (`SceneComponent.SetVisibility` _controlpanel false true))

(fn `Delete`
  (`self.Destroy`)
  (`self.K2_DestroyActor`))

(fn `Destroy`
  (`/Engine/EditorBlueprintResources/StandardMacros.DecrementInt` (`/Game/Capitality/Blueprints/BP_Factory.Operators` (`self.Factory`))))

(fn `Rotate`
  (bind _controlpanel (`self.ControlPanel`))
  (`self.K2_AddActorLocalRotation` (struct :`Yaw` 90.0))
  (`/Engine/EditorBlueprintResources/StandardMacros.IsValid` _controlpanel
    (:`Is Valid`
      (`SceneComponent.K2_AddLocalRotation` _controlpanel (struct :`Yaw` -90.0) false false)
      (set `self.AutocloseTime` (`self.GetGameTimeSinceCreation`)))))

(fn `SetButtonBlock`
  (params (Actor :type "ChildActorComponent Object Reference"))
  (bind _asbp_button_block_control (cast `/Game/Capitality/Blueprints/BP_Button_BlockControl` (`ChildActorComponent.ChildActor` Actor)))
  (set `/Game/Capitality/Blueprints/BP_Button_BlockControl.HostBlock` self _asbp_button_block_control))

(fn `UpdateAutoclose`
  (if (and (> (`self.ControlPanelSize`) 0.5) (> (- (`self.GetGameTimeSinceCreation`) (`self.AutocloseTime`)) 1.75))
    (set `self.ControlPanelSize` 0.0)))

(fn `UpdateScale`
  (params (Delta :type "Float (double-precision)"))
  (bind _controlpanelsize (`self.ControlPanelSize`))
  (bind _controlpanel (`self.ControlPanel`))
  (`SceneComponent.SetRelativeScale3D` _controlpanel (`KismetMathLibrary.VLerp` (`SceneComponent.RelativeScale3D` _controlpanel) (`KismetMathLibrary.MakeVector` _controlpanelsize _controlpanelsize _controlpanelsize) (* Delta (`self.ControlPanelTransitionSpeed`)))))

(fn `UpdateVisibility`
  (`SceneComponent.SetVisibility` (`self.ControlPanel`) (> (`KismetMathLibrary.VSize` (`SceneComponent.RelativeScale3D` (`self.ControlPanel`))) 0.05) true))

(fn `UserConstructionScript`
  (`|ExecutionSequence`
    (:`then_0`
      (bind _outactors (`GameplayStatics.GetAllActorsOfClass` "/Game/Capitality/Blueprints/BP_Factory.BP_Factory_C"))
      (for _array_element _outactors
        (bind _asbp_factory (cast `/Game/Capitality/Blueprints/BP_Factory` _array_element))
        (set `self.Factory` _asbp_factory)))
    (:`then_1`
      (`SceneComponent.SetVisibility` (`self.ControlPanel`) false true))
    (:`then_2`
      (`self.SetButtonBlock` (`self.ButtonRotate`))
      (`self.SetButtonBlock` (`self.ButtonDelete`))
      (`self.SetButtonBlock` (`self.ButtonClose`)))
    (:`then_3`
      (`TextRenderComponent.K2_SetText` (`self.TextRender`) (`self.Name`))
      (`TextRenderComponent.K2_SetText` (`self.TextRender1`) (`self.Name`))
      (`TextRenderComponent.K2_SetText` (`self.TextRender2`) (`self.Name`))
      (`TextRenderComponent.K2_SetText` (`self.TextRender3`) (`self.Name`)))))