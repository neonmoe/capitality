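; BP_Button_ControlPanel is an interactable button on a control panel that spawns a configured Block actor at the panel's transform, then closes the panel.
; Construction sets its title and subtitle text and creates a dynamic material instance, caching the default emissive color.
; Hover and Unhover swap that emissive color as highlight feedback.
; Interact records the time and triggers the spawn, while Tick animates a sine-curve press dip.
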(event `/Game/VRUUM/Blueprints/BPI_Interactible.Unhover`
  (params (Hand :type "SceneComponent Object Reference"))
  (`MaterialInstanceDynamic.SetVectorParameterValue` (`self.ButtonDMI`) "EmissiveColor" (`self.DefaultButtonColor`)))

(event `/Game/VRUUM/Blueprints/BPI_Interactible.Hover`
  (params (Hand :type "SceneComponent Object Reference"))
  (`MaterialInstanceDynamic.SetVectorParameterValue` (`self.ButtonDMI`) "EmissiveColor" (make `LinearColor` 0.3 0.4 0.9 1.0)))

(event `/Game/VRUUM/Blueprints/BPI_Interactible.Interact`
  (`parent.Interact`)
  (set `self.InteractTime` (`self.GetGameTimeSinceCreation`))
  (`self.Trigger`))

(event `self.ReceiveTick`
  (params (DeltaSeconds :type "Float (single-precision)"))
  (bind _interactanimationlength (`self.InteractAnimationLength`))
  (bind _returnvalue (- (`self.GetGameTimeSinceCreation`) (`self.InteractTime`)))
  (if (and (> _returnvalue 0.0) (< _returnvalue _interactanimationlength))
    (`SceneComponent.K2_SetRelativeLocation` (`self.Button`) (`KismetMathLibrary.MakeVector` 0.0 0.0 (* (`KismetMathLibrary.Sin` (`KismetMathLibrary.MultiplyByPi` (/ _returnvalue _interactanimationlength))) (`self.InteractAnimationDistance`) -1.0)) false false)))

(fn `Trigger`
  (bind _block (`self.Block`))
  (bind _controlpanel (`self.ControlPanel`))
  (if (`KismetSystemLibrary.IsValidClass` _block)
    (`|SpawnActorFromClass` _block (`self.GetTransform` (`self.ControlPanel`)) "Undefined" "OverrideRootScale" null null))
  (`/Engine/EditorBlueprintResources/StandardMacros.IsValid` _controlpanel
    (:`Is Valid`
      (`/Game/Capitality/Blueprints/BP_FactoryTile.Close` _controlpanel))))

(fn `UpdateText`
  (`TextRenderComponent.K2_SetText` (`self.MainText`) (`self.HeaderContent`))
  (`TextRenderComponent.K2_SetText` (`self.Subtitle`) (`self.SubtitleContent`)))

(fn `UserConstructionScript`
  (`parent.UserConstructionScript`)
  (`self.UpdateText`)
  (bind _returnvalue (`PrimitiveComponent.CreateDynamicMaterialInstance` (`self.Button`) 0 null))
  (bind _output_get (set `self.ButtonDMI` _returnvalue))
  (bind _returnvalue_2 (`MaterialInstanceDynamic.K2_GetVectorParameterValue` _output_get "EmissiveColor"))
  (set `self.DefaultButtonColor` _returnvalue_2))