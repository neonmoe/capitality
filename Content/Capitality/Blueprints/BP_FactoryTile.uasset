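; BP_FactoryTile is an interactable, non-grabbable factory tile with a pop-up control panel of buttons for Conveyor, Bouncer, Upscale, Combiner, Downscale, Color and Close.
; Construction finds the BP_Factory, hides the panel and registers the tile with each button.
; Lookedat shows and rotates the panel, then has the factory close the last one.
; Tick eases panel scale toward a target that Close zeroes, hiding it when tiny.
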(event `/Game/VRUUM/Blueprints/BPI_Interactible.LookedAt`
  (params (Rotation :type "Rotator Structure"))
  (bind _controlpanel (`self.ControlPanel`))
  (set `self.ControlPanelSize` 1.0)
  (`SceneComponent.SetVisibility` _controlpanel true true)
  (`SceneComponent.SetRelativeScale3D` _controlpanel (0.05 0.05 0.05))
  (`SceneComponent.K2_SetWorldRotation` _controlpanel Rotation false true)
  (`/Game/Capitality/Blueprints/BP_Factory.CloseLastControlPanel` (`self.Factory`) self))

(event `self.ReceiveTick`
  (params (DeltaSeconds :type "Float (single-precision)"))
  (bind _controlpanelsize (`self.ControlPanelSize`))
  (bind _controlpanel (`self.ControlPanel`))
  (`SceneComponent.SetRelativeScale3D` _controlpanel (`KismetMathLibrary.VLerp` (`SceneComponent.RelativeScale3D` _controlpanel) (`KismetMathLibrary.MakeVector` _controlpanelsize _controlpanelsize _controlpanelsize) (* DeltaSeconds (`self.ControlPanelTransitionSpeed`))))
  (`SceneComponent.SetVisibility` (`self.ControlPanel`) (> (`KismetMathLibrary.VSize` (`SceneComponent.RelativeScale3D` (`self.ControlPanel`))) 0.05) true))

(fn `CanGrab`
  (returns (Grabbability :type Boolean))
  (return false))

(fn `CanInteract`
  (returns (Interactiblity :type Boolean))
  (return true))

(fn `Close`
  (set `self.ControlPanelSize` 0.0))

(fn `SetButtonControlPanel`
  (params (Actor :type "ChildActorComponent Object Reference"))
  (bind _asbp_button_control_panel (cast `/Game/Capitality/Blueprints/BP_Button_ControlPanel` (`ChildActorComponent.ChildActor` Actor)))
  (set `/Game/Capitality/Blueprints/BP_Button_ControlPanel.ControlPanel` self _asbp_button_control_panel))

(fn `UserConstructionScript`
  (bind _controlpanel (`self.ControlPanel`))
  (bind _outactors (`GameplayStatics.GetAllActorsOfClass` "/Game/Capitality/Blueprints/BP_Factory.BP_Factory_C"))
  (for _array_element _outactors
    (set `self.Factory` _array_element))
  (`SceneComponent.SetVisibility` _controlpanel false true)
  (`SceneComponent.SetRelativeScale3D` _controlpanel (0.0 0.0 0.0))
  (`self.SetButtonControlPanel` (`self.ButtonConveyor`))
  (`self.SetButtonControlPanel` (`self.ButtonBouncer`))
  (`self.SetButtonControlPanel` (`self.ButtonUpscale`))
  (`self.SetButtonControlPanel` (`self.ButtonCombiner`))
  (`self.SetButtonControlPanel` (`self.ButtonDownscale`))
  (`self.SetButtonControlPanel` (`self.ButtonColor`))
  (`self.SetButtonControlPanel` (`self.ButtonClose`)))