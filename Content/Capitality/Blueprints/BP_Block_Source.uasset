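; BP_Block_Source is a factory block that emits props while its Factory has spawning enabled.
; On Tick it compares time since creation to the last spawn time, creating a BP_Prop at SpawnPoint at a fixed interval of just over two seconds.
; Each prop gets a mass-independent impulse forward and upward, then is added to the Factory's Props list.
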(event `self.ReceiveTick`
  (params (DeltaSeconds :type "Float (single-precision)"))
  (bind _returnvalue (`self.GetGameTimeSinceCreation`))
  (`parent.ReceiveTick` DeltaSeconds)
  (if (and (> (- _returnvalue (`self.LastSpawnTime`)) 2.0) (`/Game/Capitality/Blueprints/BP_Factory.Spawning` (`self.Factory`)))
    (set `self.LastSpawnTime` _returnvalue)
    (bind _returnvalue_2 (`|SpawnActorFromClass` "/Game/Capitality/Blueprints/BP_Prop.BP_Prop_C" (`KismetMathLibrary.MakeTransform` (`SceneComponent.K2_GetComponentLocation` (`self.SpawnPoint`))) "Undefined" "OverrideRootScale" null null))
    (`PrimitiveComponent.AddImpulse` (`StaticMeshActor.StaticMeshComponent` _returnvalue_2) (+ (* (`self.GetActorForwardVector`) 150.0) (0.0 0.0 250.0)) "None" true)
    (`KismetArrayLibrary.Array_Add` (`/Game/Capitality/Blueprints/BP_Factory.Props` (`self.Factory`)) _returnvalue_2)))

(fn `UserConstructionScript`
  (`parent.UserConstructionScript`))