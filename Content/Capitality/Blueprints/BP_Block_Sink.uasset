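; BP_Block_Sink is a block that consumes props and converts them into points for a Factory.
; When an actor begins overlapping its Sink component, it casts to BP_Prop and ignores anything else.
; Each matching prop is destroyed, and a small random integer is added to the referenced Factory's Points.
; Tick is disabled and the construction script only calls its parent.
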(event `self.Sink.OnComponentBeginOverlap`
  (params (OverlappedComponent :type "PrimitiveComponent Object Reference") (OtherActor :type "Actor Object Reference") (OtherComp :type "PrimitiveComponent Object Reference") (OtherBodyIndex :type Integer) (bFromSweep :type Boolean) (SweepResult :type "HitResult Structure (by ref)"))
  (bind _factory (`self.Factory`))
  (bind _asbp_prop (cast `/Game/Capitality/Blueprints/BP_Prop` OtherActor))
  (`self.K2_DestroyActor` _asbp_prop)
  (set `/Game/Capitality/Blueprints/BP_Factory.Points` (+ (`/Game/Capitality/Blueprints/BP_Factory.Points` _factory) (`KismetMathLibrary.RandomIntegerInRange` 1 10)) _factory))

(fn `UserConstructionScript`
  (`parent.UserConstructionScript`))