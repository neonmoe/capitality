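; BP_HandVR is a VR hand actor that handles teleport aiming, pointing and grab forwarding.
; Tick predicts a projectile arc, validates its landing on the navmesh and rebuilds spline meshes colored by validity.
; In its pointing state, a Pawn-only trace sends LookedAt messages to BPI_Interactible actors.
; Grab and Ungrab message hovered interactibles, but the overlap logic that fills that list is disconnected.
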(event `self.ReceiveActorBeginOverlap`
  (params (OtherActor :type "Actor Object Reference")))

(event `self.ReceiveActorEndOverlap`
  (params (OtherActor :type "Actor Object Reference")))

(event `self.ReceiveTick`
  (params (DeltaSeconds :type "Float (single-precision)"))
  (`self.UpdateTeleport`)
  (`self.UpdatePointing`)
  (if (>= (- (`self.GetGameTimeSinceCreation`) (`self.HoverDisableTime`)) 0.1)
    (set `PrimitiveComponent.bGenerateOverlapEvents` true (`self.Collider`))))

(fn `ClearSplineMeshes`
  (bind _splinemeshes (`self.SplineMeshes`))
  (`ActorComponent.K2_DestroyComponent` _splinemeshes)
  (`KismetArrayLibrary.Array_Clear` _splinemeshes))

(fn `Grab`
  (for _array_element (`self.HoveredInteractibles`)
    (message `/Game/VRUUM/Blueprints/BPI_Interactible.Grab` _array_element (`self.Collider`))))

(fn `StateIs`
  (params (State :type "/Game/VRUUM/Blueprints/EHandState Enum" :default "NewEnumerator0"))
  (returns (IsEqual :type Boolean))
  (return (`|EnumEquality` (`self.State`) State)))

(fn `Ungrab`
  (for _array_element (`self.HoveredInteractibles`)
    (message `/Game/VRUUM/Blueprints/BPI_Interactible.Ungrab` _array_element (`self.Collider`))))

(fn `UpdatePointing`
  (bind _returnvalue (`SceneComponent.K2_GetComponentLocation` (`self.PointingOffset`)))
  (bind _isequal (`self.StateIs` "NewEnumerator2"))
  (if _isequal
    (bind (_outhit _returnvalue_2) (`KismetSystemLibrary.LineTraceSingleForObjects` :`Start` _returnvalue :`End` (+ _returnvalue (* (`SceneComponent.GetForwardVector` (`self.Hand`)) 300.0)) :`ObjectTypes` (`|MakeArray` "ObjectTypeQuery3" :!type "EObjectTypeQuery Enum") :`DrawTime` 0.5))
    (if _returnvalue_2
      (bind (_bblockinghit _binitialoverlap _time _distance _location _impactpoint _normal _impactnormal _physmat _hitactor) (`GameplayStatics.BreakHitResult` _outhit))
      (if (and (`KismetSystemLibrary.DoesImplementInterface` _hitactor "/Game/VRUUM/Blueprints/BPI_Interactible.BPI_Interactible_C") (!= _hitactor (`self.LastPointedActor`)))
        (set `self.LastPointedActor` _hitactor)
        (message `/Game/VRUUM/Blueprints/BPI_Interactible.LookedAt` _hitactor (`KismetMathLibrary.FindLookAtRotation` (`KismetMathLibrary.MakeVector` (.x (`self.K2_GetActorLocation` _hitactor)) (.y (`self.K2_GetActorLocation` _hitactor))) (`KismetMathLibrary.MakeVector` (.x (`self.K2_GetActorLocation`)) (.y (`self.K2_GetActorLocation`))))))
      (else
        (set `self.LastPointedActor` null)))))

(fn `UpdateSplineColor`
  (for _array_element (`self.SplineMeshes`)
    (bind _returnvalue (`PrimitiveComponent.CreateDynamicMaterialInstance` _array_element 0 (`PrimitiveComponent.GetMaterial` _array_element 0)))
    (if (`self.CanTeleport`)
      (`MaterialInstanceDynamic.SetVectorParameterValue` _returnvalue "Color" (`KismetMathLibrary.Conv_ColorToLinearColor` (`self.TeleportColorDefault`)))
      (else
        (`MaterialInstanceDynamic.SetVectorParameterValue` _returnvalue "Color" (`KismetMathLibrary.Conv_ColorToLinearColor` (`self.TeleportColorDisabled`)))))))

(fn `UpdateSplineMeshes`
  (params (Positions :type "Array of Vector Structure"))
  (bind _teleportarc (`self.TeleportArc`))
  (for _index (range (+ (- (`KismetArrayLibrary.Array_Length` Positions) 2) 1))
    (`SplineComponent.AddSplinePoint` _teleportarc (`|GetArrayItem` Positions _index) "World" false)
    (bind _returnvalue (`AddComponent|NODE_AddSplineMeshComponent-1` :`bManualAttachment` true))
    (`PrimitiveComponent.SetMaterial` _returnvalue 0 "/Game/VRUUM/Art/TeleportArc/M_TeleportArc.M_TeleportArc")
    (bind _returnvalue_2 (+ _index 1))
    (`SplineMeshComponent.SetStartAndEnd` _returnvalue (`|GetArrayItem` Positions _index) (`SplineComponent.GetTangentAtSplinePoint` _teleportarc _index "Local") (`|GetArrayItem` Positions _returnvalue_2) (`SplineComponent.GetTangentAtSplinePoint` _teleportarc _returnvalue_2 "Local") true)
    (`KismetArrayLibrary.Array_Add` (`self.SplineMeshes`) _returnvalue))
  (`SplineComponent.SetSplinePointType` _teleportarc (`KismetArrayLibrary.Array_LastIndex` Positions) "CurveClamped" true))

(fn `UpdateTeleport`
  (locals (TeleportLaunchVelocity :type "Float (double-precision)" :default 1000.0) (Positions :type "Array of Vector Structure"))
  (`SplineComponent.ClearSplinePoints` (`self.TeleportArc`) true)
  (`self.ClearSplineMeshes`)
  (if (`self.Teleporting`)
    (bind (_outhit _outpathpositions _outlasttracedestination _returnvalue) (`GameplayStatics.Blueprint_PredictProjectilePath_ByObjectType` :`StartPos` (`SceneComponent.K2_GetComponentLocation` (`self.TeleportArc`)) :`LaunchVelocity` (* (`SceneComponent.GetForwardVector` (`self.Hand`)) (`local.TeleportLaunchVelocity`)) :`ProjectileRadius` 5.0 :`ObjectTypes` (`|MakeArray` "ObjectTypeQuery1" "ObjectTypeQuery2" :!type "EObjectTypeQuery Enum") :`SimFrequency` 30.0)) ; Simulate throwing a projectile (including gravity) to find a teleport location.
    (bind (_bblockinghit _binitialoverlap _time _distance _location) (`GameplayStatics.BreakHitResult` _outhit))
    (set `self.TeleportPoint` _location)
    (`self.UpdateSplineMeshes` _outpathpositions)
    (bind (_projectedlocation _returnvalue_2) (`NavigationSystem.K2_ProjectPointToNavigation` _location null null (30.0 30.0 30.0)))
    (set `self.CanTeleport` (and _returnvalue _returnvalue_2))
    (`self.UpdateSplineColor`)
    (set `self.TeleportPointNav` _projectedlocation)))

(fn `UserConstructionScript`)