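; VR player pawn that turns motion controller input into grabbing, trigger and thumbstick teleport actions for two BP_HandVR child actors.
; Each hand's state enum gates input, so actions start only from the default state.
; Tick moves each teleport marker to its hand's target, recoloring a dynamic material by validity.
; Releasing the thumbstick teleports to the hand's nav point, offset by HMD horizontal position, with sound.
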(event `Key|MotionController_Right_Trigger`
  (params (Key :type "Key Structure"))
  (:`Pressed`
    (bind _idle (`self.IsRight` "NewEnumerator0"))
    (if _idle
      (`self.SetStateFromHand` "Right" "NewEnumerator2")))
  (:`Released`
    (bind _idle_2 (`self.IsRight` "NewEnumerator2"))
    (if _idle_2
      (`self.SetStateFromHand` "Right"))))

(event `self.ReceiveTick`
  (params (DeltaSeconds :type "Float (single-precision)"))
  (bind _hand (`self.GetLeftHand`))
  (`self.UpdateTeleportPoint` (`self.LeftTeleportPoint`) _hand (`self.LeftTeleportPointMI`))
  (bind _hand_2 (`self.GetRightHand`))
  (`self.UpdateTeleportPoint` (`self.RightTeleportPoint`) _hand_2 (`self.RightTeleportPointMI`)))

(event `Key|MotionController_Left_Grip1`
  (params (Key :type "Key Structure"))
  (bind _lefthandbp (`self.LeftHandBP`))
  (:`Pressed`
    (`self.Grab` _lefthandbp :!label _label))
  (:`Released`
    (`self.Ungrab` _lefthandbp :!label _label_2)))

(event `Key|MotionController_Right_Grip1`
  (params (Key :type "Key Structure"))
  (bind _righthandbp (`self.RightHandBP`))
  (:`Pressed`
    (`self.Grab` _righthandbp "Right" :!label _label_3))
  (:`Released`
    (`self.Ungrab` _righthandbp "Right" :!label _label_4)))

(event `Key|MotionController_Left_Trigger`
  (params (Key :type "Key Structure"))
  (:`Pressed`
    (bind _idle (`self.IsLeft` "NewEnumerator0"))
    (if _idle
      (`self.SetStateFromHand` "Left" "NewEnumerator2")))
  (:`Released`
    (bind _idle_2 (`self.IsLeft` "NewEnumerator2"))
    (if _idle_2
      (`self.SetStateFromHand` "Left"))))

(event `Key|MotionController_Left_Grip2`
  (params (Key :type "Key Structure"))
  (:`Pressed`
    (goto _label))
  (:`Released`
    (goto _label_2)))

(event `Key|MotionController_Right_Grip2`
  (params (Key :type "Key Structure"))
  (:`Pressed`
    (goto _label_3))
  (:`Released`
    (goto _label_4)))

(event `Key|MotionController_Right_Thumbstick`
  (params (Key :type "Key Structure"))
  (:`Pressed`
    (bind _idle (`self.IsRight` "NewEnumerator0"))
    (if _idle
      (bind _hand (`self.GetRightHand`))
      (set `/Game/VRUUM/Blueprints/BP_HandVR.Teleporting` true _hand)
      (`AudioComponent.Play` (`self.RightTeleportInitSoundFx`) 0.0)
      (`self.SetStateFromHand` "Right" "NewEnumerator3")))
  (:`Released`
    (bind _idle_2 (`self.IsRight` "NewEnumerator3"))
    (if _idle_2
      (bind _hand_2 (`self.GetRightHand`))
      (`self.TeleportTo` _hand_2 (`self.RightTeleportSoundFx`))
      (`self.SetStateFromHand` "Right"))))

(event `Key|MotionController_Left_Thumbstick`
  (params (Key :type "Key Structure"))
  (:`Pressed`
    (bind _idle (`self.IsLeft` "NewEnumerator0"))
    (if _idle
      (bind _hand (`self.GetLeftHand`))
      (set `/Game/VRUUM/Blueprints/BP_HandVR.Teleporting` true _hand)
      (`AudioComponent.Play` (`self.LeftTeleportInitSoundFx`) 0.0)
      (`self.SetStateFromHand` "Left" "NewEnumerator3")))
  (:`Released`
    (bind _idle_2 (`self.IsLeft` "NewEnumerator3"))
    (if _idle_2
      (bind _hand_2 (`self.GetLeftHand`))
      (`self.TeleportTo` _hand_2 (`self.LeftTeleportSoundFx`))
      (`self.SetStateFromHand` "Left"))))

(fn `GetLeftHand`
  (returns (Hand :type "/Game/VRUUM/Blueprints/BP_HandVR Object Reference"))
  (bind _asbp_hand_vr (cast `/Game/VRUUM/Blueprints/BP_HandVR` (`ChildActorComponent.ChildActor` (`self.LeftHandBP`))))
  (return _asbp_hand_vr))

(fn `GetRightHand`
  (returns (Hand :type "/Game/VRUUM/Blueprints/BP_HandVR Object Reference"))
  (bind _asbp_hand_vr (cast `/Game/VRUUM/Blueprints/BP_HandVR` (`ChildActorComponent.ChildActor` (`self.RightHandBP`))))
  (return _asbp_hand_vr))

(fn `GetStateFromHand`
  (params (Hand :type "EControllerHand Enum" :default "Left"))
  (returns (State :type "/Game/VRUUM/Blueprints/EHandState Enum"))
  (if (`|EnumEquality` Hand "Left")
    (bind _hand (`self.GetLeftHand`))
    (return (`/Game/VRUUM/Blueprints/BP_HandVR.State` _hand))
    (else
      (bind _hand_2 (`self.GetRightHand`))
      (return (`/Game/VRUUM/Blueprints/BP_HandVR.State` _hand_2)))))

(fn `Grab`
  (params (HandActor :type "ChildActorComponent Object Reference") (Hand :type "EControllerHand Enum" :default "Left"))
  (bind _asbp_hand_vr (cast `/Game/VRUUM/Blueprints/BP_HandVR` (`ChildActorComponent.ChildActor` HandActor)))
  (bind _state (`self.GetStateFromHand` Hand))
  (if (`|EnumEquality` _state "NewEnumerator0")
    (`/Game/VRUUM/Blueprints/BP_HandVR.Grab` _asbp_hand_vr)
    (`self.SetStateFromHand` Hand "NewEnumerator1")))

(fn `IsLeft`
  (params (State :type "/Game/VRUUM/Blueprints/EHandState Enum" :default "NewEnumerator0"))
  (returns (Idle :type Boolean))
  (bind _hand (`self.GetLeftHand`))
  (return (`|EnumEquality` (`/Game/VRUUM/Blueprints/BP_HandVR.State` _hand) State)))

(fn `IsRight`
  (params (State :type "/Game/VRUUM/Blueprints/EHandState Enum" :default "NewEnumerator0"))
  (returns (Idle :type Boolean))
  (bind _hand (`self.GetRightHand`))
  (return (`|EnumEquality` (`/Game/VRUUM/Blueprints/BP_HandVR.State` _hand) State)))

(fn `SetStateFromHand`
  (params (Hand :type "EControllerHand Enum" :default "Left") (State :type "/Game/VRUUM/Blueprints/EHandState Enum" :default "NewEnumerator0"))
  (if (`|EnumEquality` Hand "Left")
    (bind _hand (`self.GetLeftHand`))
    (set `/Game/VRUUM/Blueprints/BP_HandVR.State` State _hand)
    (else
      (bind _hand_2 (`self.GetRightHand`))
      (set `/Game/VRUUM/Blueprints/BP_HandVR.State` State _hand_2))))

(fn `TeleportTo`
  (params (Hand :type "/Game/VRUUM/Blueprints/BP_HandVR Object Reference") (Sound :type "AudioComponent Object Reference"))
  (set `/Game/VRUUM/Blueprints/BP_HandVR.Teleporting` false Hand)
  (if (`/Game/VRUUM/Blueprints/BP_HandVR.CanTeleport` Hand)
    (`self.K2_TeleportTo` (- (`/Game/VRUUM/Blueprints/BP_HandVR.TeleportPointNav` Hand) (`KismetMathLibrary.MakeVector` (.x (`.DevicePosition` (`HeadMountedDisplayFunctionLibrary.GetOrientationAndPosition`))) (.y (`.DevicePosition` (`HeadMountedDisplayFunctionLibrary.GetOrientationAndPosition`))))) (`self.K2_GetActorRotation`))
    (`AudioComponent.Play` Sound 0.0)))

(fn `Ungrab`
  (params (HandActor :type "ChildActorComponent Object Reference") (Hand :type "EControllerHand Enum" :default "Left"))
  (bind _asbp_hand_vr (cast `/Game/VRUUM/Blueprints/BP_HandVR` (`ChildActorComponent.ChildActor` HandActor)))
  (bind _state (`self.GetStateFromHand` Hand))
  (if (`|EnumEquality` _state "NewEnumerator1")
    (`/Game/VRUUM/Blueprints/BP_HandVR.Ungrab` _asbp_hand_vr)
    (`self.SetStateFromHand` Hand)))

(fn `UpdateTeleportPoint`
  (params (Point :type "StaticMeshComponent Object Reference") (Hand :type "/Game/VRUUM/Blueprints/BP_HandVR Object Reference") (MaterialInstance :type "MaterialInstanceDynamic Object Reference"))
  (if (`/Game/VRUUM/Blueprints/BP_HandVR.Teleporting` Hand)
    (`SceneComponent.SetVisibility` Point true false)
    (`SceneComponent.K2_SetWorldLocation` Point (`/Game/VRUUM/Blueprints/BP_HandVR.TeleportPoint` Hand) false false)
    (if (`/Game/VRUUM/Blueprints/BP_HandVR.CanTeleport` Hand)
      (`MaterialInstanceDynamic.SetVectorParameterValue` MaterialInstance "Color" (`KismetMathLibrary.Conv_ColorToLinearColor` (`self.TeleportPointColorDefault`)))
      (else
        (`MaterialInstanceDynamic.SetVectorParameterValue` MaterialInstance "Color" (`KismetMathLibrary.Conv_ColorToLinearColor` (`self.TeleportPointColorDisabled`)))))
    (else
      (`SceneComponent.SetVisibility` Point false false))))

(fn `UserConstructionScript`
  (bind _leftteleportpoint (`self.LeftTeleportPoint`))
  (bind _rightteleportpoint (`self.RightTeleportPoint`))
  (bind _returnvalue (`PrimitiveComponent.CreateDynamicMaterialInstance` _leftteleportpoint 0 (`PrimitiveComponent.GetMaterial` _leftteleportpoint 0)))
  (set `self.LeftTeleportPointMI` _returnvalue)
  (bind _returnvalue_2 (`PrimitiveComponent.CreateDynamicMaterialInstance` _rightteleportpoint 0 (`PrimitiveComponent.GetMaterial` _rightteleportpoint 0)))
  (set `self.RightTeleportPointMI` _returnvalue_2)
  (bind _hand (`self.GetLeftHand`))
  (set `/Game/VRUUM/Blueprints/BP_HandVR.TeleportColorDefault` (`self.TeleportPointColorDefault`) _hand)
  (set `/Game/VRUUM/Blueprints/BP_HandVR.TeleportColorDisabled` (`self.TeleportPointColorDisabled`) _hand)
  (bind _hand_2 (`self.GetRightHand`))
  (set `/Game/VRUUM/Blueprints/BP_HandVR.TeleportColorDefault` (`self.TeleportPointColorDefault`) _hand_2)
  (set `/Game/VRUUM/Blueprints/BP_HandVR.TeleportColorDisabled` (`self.TeleportPointColorDisabled`) _hand_2))