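; Base pickupable actor that a hand can grab and release, with a hover indicator.
; Grab disables mesh physics and attaches the actor to the hand; Ungrab restores physics and detaches.
; Construction adds an invisible, shrunken mesh copy with blocking collision, and sizes the indicator to the mesh's horizontal bounds, or zero when an HMD is enabled.
; Tick shows the indicator with zeroed world rotation while hovered, unless hidden.
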(event `/Game/VRUUM/Blueprints/BPI_Interactible.Grab`
  (params (Hand :type "SceneComponent Object Reference"))
  (`PrimitiveComponent.SetSimulatePhysics` (`self.StaticMeshComponent`) false)
  (`SceneComponent.K2_AttachToComponent` (`self.RootComponent`) Hand "None" "KeepWorld" "KeepWorld" "KeepWorld" false))

(event `/Game/VRUUM/Blueprints/BPI_Interactible.Ungrab`
  (params (Hand :type "SceneComponent Object Reference"))
  (`PrimitiveComponent.SetSimulatePhysics` (`self.StaticMeshComponent`) true)
  (`self.K2_DetachFromActor` "KeepWorld" "KeepWorld" "KeepWorld"))

(event `self.ReceiveTick`
  (params (DeltaSeconds :type "Float (single-precision)"))
  (`self.UpdateHoverIndicator`))

(event `/Game/VRUUM/Blueprints/BPI_Interactible.Hover`
  (params (Hand :type "SceneComponent Object Reference"))
  (set `self.Hovered` true))

(event `/Game/VRUUM/Blueprints/BPI_Interactible.Unhover`
  (params (Hand :type "SceneComponent Object Reference"))
  (set `self.Hovered` false))

(fn `CanGrab`
  (returns (Grabbability :type Boolean))
  (return true))

(fn `CanInteract`
  (returns (Interactiblity :type Boolean))
  (return false))

(fn `UpdateHoverIndicator`
  (bind _indicator (`self.Indicator`))
  (if (and (`self.Hovered`) (not (`self.HideHoverIndicator`)))
    (`SceneComponent.SetVisibility` _indicator true false)
    (`SceneComponent.K2_SetWorldRotation` :`self` _indicator)
    (else
      (`SceneComponent.SetVisibility` _indicator false false))))

(fn `UserConstructionScript`
  (bind _indicator (`self.Indicator`))
  (bind _returnvalue (* (`KismetMathLibrary.FMax` (.x (`.BoxExtent` (`KismetSystemLibrary.GetComponentBounds` (`self.StaticMeshComponent`)))) (.y (`.BoxExtent` (`KismetSystemLibrary.GetComponentBounds` (`self.StaticMeshComponent`))))) 1.0))
  (bind _returnvalue_2 (`AddComponent|NODE_AddStaticMeshComponent-0` :`RelativeTransform` (`KismetMathLibrary.MakeTransform` (0.0 0.0 0.0) (struct) (0.7 0.7 0.7))))
  (`StaticMeshComponent.SetStaticMesh` _returnvalue_2 (`StaticMeshComponent.StaticMesh` (`self.StaticMeshComponent`)))
  (`PrimitiveComponent.SetCollisionResponseToAllChannels` _returnvalue_2 "ECR_Block")
  (`PrimitiveComponent.SetCollisionObjectType` _returnvalue_2 "ECC_WorldDynamic")
  (`SceneComponent.SetVisibility` _returnvalue_2 false false)
  (if (`HeadMountedDisplayFunctionLibrary.IsHeadMountedDisplayEnabled`)
    (`SceneComponent.SetRelativeScale3D` _indicator (0.0 0.0 0.0))
    (else
      (`SceneComponent.SetRelativeScale3D` _indicator (`KismetMathLibrary.MakeVector` _returnvalue _returnvalue _returnvalue)))))