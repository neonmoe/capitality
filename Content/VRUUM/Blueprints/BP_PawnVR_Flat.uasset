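; Flatscreen player pawn that walks, looks around and interacts with or grabs objects without VR input.
; Each tick it applies camera-relative horizontal movement and runs a short camera line trace against Pawn-type objects implementing BPI_Interactible, sending hover and unhover messages.
; The hovered actor drives HUD tooltips and receives Interact and Grab/Ungrab interface messages, with Interact also sending it a flattened rotation toward the camera.
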(event `self.ReceiveBeginPlay`
  (bind _returnvalue (`|CreateWidget` "/Game/VRUUM/UI/WBP_FlatscreenHUD.WBP_FlatscreenHUD_C"))
  (bind _output_get (set `self.HUD` _returnvalue))
  (`UserWidget.AddToViewport` _output_get 0))

(event `self.ReceiveTick`
  (params (DeltaSeconds :type "Float (single-precision)"))
  (`self.Move`)
  (`self.UpdateHoveredStatus`)
  (`self.UpdateHUD`))

(event `InputAxis|LookUp`
  (params (AxisValue :type "Float (single-precision)"))
  (`self.AddControllerPitchInput` AxisValue))

(event `InputAxis|LookRight`
  (params (AxisValue :type "Float (single-precision)"))
  (`self.AddControllerYawInput` AxisValue))

(event `InputAction|Interact`
  (params (Key :type "Key Structure"))
  (bind _hoveredactor (`self.HoveredActor`))
  (:`Pressed`
    (`/Engine/EditorBlueprintResources/StandardMacros.IsValid` _hoveredactor
      (:`Is Valid`
        (message `/Game/VRUUM/Blueprints/BPI_Interactible.Interact` _hoveredactor)
        (`/Engine/EditorBlueprintResources/StandardMacros.IsValid` _hoveredactor
          (:`Is Valid`
            (message `/Game/VRUUM/Blueprints/BPI_Interactible.LookedAt` _hoveredactor (`KismetMathLibrary.FindLookAtRotation` (`KismetMathLibrary.MakeVector` (.x (`self.K2_GetActorLocation` _hoveredactor)) (.y (`self.K2_GetActorLocation` _hoveredactor))) (`KismetMathLibrary.MakeVector` (.x (`SceneComponent.K2_GetComponentLocation` (`self.Camera`))) (.y (`SceneComponent.K2_GetComponentLocation` (`self.Camera`))))))))))))

(event `InputAction|Grab`
  (params (Key :type "Key Structure"))
  (bind _hoveredactor (`self.HoveredActor`))
  (bind _hand (`self.Hand`))
  (:`Pressed`
    (message `/Game/VRUUM/Blueprints/BPI_Interactible.Grab` _hoveredactor _hand))
  (:`Released`
    (message `/Game/VRUUM/Blueprints/BPI_Interactible.Ungrab` _hoveredactor _hand)))

(fn `Move`
  (bind _camera (`self.Camera`))
  (`PawnMovementComponent.AddInputVector` (`self.CharacterMovement`) (`KismetMathLibrary.Normal` (+ (* (`KismetMathLibrary.Normal` (`KismetMathLibrary.MakeVector` (.x (`SceneComponent.GetForwardVector` _camera)) (.y (`SceneComponent.GetForwardVector` _camera)))) (`self.GetInputAxisValue`)) (* (`KismetMathLibrary.Normal` (`SceneComponent.GetRightVector` _camera)) (`self.GetInputAxisValue`)))) false))

(fn `UpdateHoveredStatus`
  (bind _hover (`self.Hover`))
  (bind _camera (`self.Camera`))
  (bind _returnvalue (`SceneComponent.K2_GetComponentLocation` _camera))
  (bind (_outhit _returnvalue_2) (`KismetSystemLibrary.LineTraceSingleForObjects` :`Start` _returnvalue :`End` (+ _returnvalue (* (`SceneComponent.GetForwardVector` _camera) 300.0)) :`ObjectTypes` (`|MakeArray` "ObjectTypeQuery3" :!type "EObjectTypeQuery Enum") :`bTraceComplex` true :`DrawTime` 0.2))
  (if _returnvalue_2
    (bind (_bblockinghit _binitialoverlap _time _distance _location _impactpoint _normal _impactnormal _physmat _hitactor) (`GameplayStatics.BreakHitResult` _outhit))
    (if (`KismetSystemLibrary.DoesImplementInterface` _hitactor "/Game/VRUUM/Blueprints/BPI_Interactible.BPI_Interactible_C")
      (if (or (!= _hitactor (`self.HoveredActor`)) (not _hover))
        (`/Engine/EditorBlueprintResources/StandardMacros.IsValid` (`self.HoveredActor`)
          (:`Is Valid`
            (message `/Game/VRUUM/Blueprints/BPI_Interactible.Unhover` (`self.HoveredActor`) null))
          (:`Is Not Valid`
            _))
        (bind _output_get (set `self.HoveredActor` _hitactor))
        (message `/Game/VRUUM/Blueprints/BPI_Interactible.Hover` _output_get null)
        (set `self.Hover` true))
      (else
        (if _hover :!label _label
          (`/Engine/EditorBlueprintResources/StandardMacros.IsValid` (`self.HoveredActor`)
            (:`Is Valid`
              (message `/Game/VRUUM/Blueprints/BPI_Interactible.Unhover` (`self.HoveredActor`) null))
            (:`Is Not Valid`
              _)))
        (set `self.Hover` false)))
    (else
      (goto _label))))

(fn `UpdateHUD`
  (if (`self.Hover`)
    (`|ExecutionSequence`
      (:`then_0`
        (bind _interactiblity (message `/Game/VRUUM/Blueprints/BPI_Interactible.CanInteract` (`self.HoveredActor`)))
        (if _interactiblity
          (`Widget.SetVisibility` (`/Game/VRUUM/UI/WBP_FlatscreenHUD.InteractTooltip` (`self.HUD`)) "Visible")))
      (:`then_1`
        (bind _grabbability (message `/Game/VRUUM/Blueprints/BPI_Interactible.CanGrab` (`self.HoveredActor`)))
        (if _grabbability
          (`Widget.SetVisibility` (`/Game/VRUUM/UI/WBP_FlatscreenHUD.GrabTooltip` (`self.HUD`)) "Visible"))))
    (else
      (`Widget.SetVisibility` (`/Game/VRUUM/UI/WBP_FlatscreenHUD.GrabTooltip` (`self.HUD`)) "Collapsed")
      (`Widget.SetVisibility` (`/Game/VRUUM/UI/WBP_FlatscreenHUD.InteractTooltip` (`self.HUD`)) "Collapsed"))))

(fn `UserConstructionScript`)