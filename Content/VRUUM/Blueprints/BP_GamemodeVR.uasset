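; BP_GamemodeVR is a game mode that spawns and possesses the player's pawn when play begins.
; It spawns BP_PawnVR_Flat at the first PlayerStart found, has player controller 0 possess it, and logs the mode.
; A head-mounted display check exists but both branches are empty, so the flat pawn is always used.
; The matching BP_PawnVR spawn-and-possess chain is disconnected and never runs.
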(event `self.ReceiveBeginPlay`
  (bind _outactors (`GameplayStatics.GetAllActorsOfClass` "/Script/Engine.PlayerStart"))
  (if (`HeadMountedDisplayFunctionLibrary.IsHeadMountedDisplayEnabled`)
    _
    (else
      _))
  (bind _returnvalue (`|SpawnActorFromClass` "/Game/VRUUM/Blueprints/BP_PawnVR_Flat.BP_PawnVR_Flat_C" (`self.GetTransform` (`|GetArrayItem` _outactors)) "AdjustIfPossibleButAlwaysSpawn" "OverrideRootScale" null null))
  (`Controller.Possess` (`GameplayStatics.GetPlayerController` 0) _returnvalue)
  (`VisualLoggerKismetLibrary.LogText` "Flat"))

(fn `UserConstructionScript`)