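; BP_Button is an interactable, non-grabbable button that triggers other objects when used.
; On Interact, it forwards the interact message to every entry in its Targets array, then plays an activation sound.
; The construction script caches the Button component's relative scale and assigns the configurable sound effect to the audio component.
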(event `/Game/VRUUM/Blueprints/BPI_Interactible.Interact`
  (for _array_element (`self.Targets`)
    (message `/Game/VRUUM/Blueprints/BPI_Interactible.Interact` _array_element))
  (`AudioComponent.Play` (`self.ActivationSound`) 0.0))

(fn `CanGrab`
  (returns (Grabbability :type Boolean))
  (return false))

(fn `CanInteract`
  (returns (Interactiblity :type Boolean))
  (return true))

(fn `UserConstructionScript`
  (set `self.BaseScale` (`SceneComponent.RelativeScale3D` (`self.Button`)))
  (`AudioComponent.SetSound` (`self.ActivationSound`) (`self.ActivationSfx`)))